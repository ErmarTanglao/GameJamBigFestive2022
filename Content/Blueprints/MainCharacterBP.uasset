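; Player character Blueprint with a basic fireball attack and three extra magic attacks gated by Obtained Blue, Brown and Green flags.
; Attack inputs spawn projectiles at ProjectileSpawn; only the fireball plays a montage and checks that the player is alive.
; AnyDamage lowers PlayerHealth and, at zero or below, sets Dead, disables collision and movement, then plays dying animations.
; BeginPlay turns off tonemapping and eye adaptation through console commands.
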(event Input|EnhancedActionEvents|EnhancedInputActionIA_Attack1
  (params (ActionValue :type Boolean) (ElapsedSeconds :type Float%20%28double-precision%29) (TriggeredSeconds :type Float%20%28double-precision%29) (InputAction :type Input%20Action%20Object%20Reference :default "/Game/Blueprints/Input/IA_Attack1.IA_Attack1"))
  (:Triggered
    (CallFunction|SpawnFireboll)))

(event Input|EnhancedActionEvents|EnhancedInputActionIA_Attack2
  (params (ActionValue :type Boolean) (ElapsedSeconds :type Float%20%28double-precision%29) (TriggeredSeconds :type Float%20%28double-precision%29) (InputAction :type Input%20Action%20Object%20Reference :default "/Game/Blueprints/Input/IA_Attack2.IA_Attack2"))
  (:Triggered
    (if (Variables|Default|GetObtainedBlue)
      (Game|SpawnActorfromClass "/Game/Characters/MainCharacter/Blueprint/BP_MagicAttack2.BP_MagicAttack2_C" (Transformation|GetWorldTransform (Variables|Default|GetProjectileSpawn)) "AlwaysSpawn" 0 self))))

(event Input|EnhancedActionEvents|EnhancedInputActionIA_Attack3
  (params (ActionValue :type Boolean) (ElapsedSeconds :type Float%20%28double-precision%29) (TriggeredSeconds :type Float%20%28double-precision%29) (InputAction :type Input%20Action%20Object%20Reference :default "/Game/Blueprints/Input/IA_Attack3.IA_Attack3"))
  (:Triggered
    (if (Variables|Default|GetObtainedBrown)
      (Game|SpawnActorfromClass "/Game/Characters/MainCharacter/Blueprint/BP_MagicAttack3.BP_MagicAttack3_C" (Transformation|GetWorldTransform (Variables|Default|GetProjectileSpawn)) "AlwaysSpawn" 0 self))))

(event Input|EnhancedActionEvents|EnhancedInputActionIA_Attack4
  (params (ActionValue :type Boolean) (ElapsedSeconds :type Float%20%28double-precision%29) (TriggeredSeconds :type Float%20%28double-precision%29) (InputAction :type Input%20Action%20Object%20Reference :default "/Game/Blueprints/Input/IA_Attack4.IA_Attack4"))
  (:Triggered
    (if (Variables|Default|GetObtainedGreen)
      (Game|SpawnActorfromClass "/Game/Characters/MainCharacter/Blueprint/BP_MagicAttack4.BP_MagicAttack4_C" (Transformation|GetWorldTransform (Variables|Default|GetProjectileSpawn)) "AlwaysSpawn" 0 self))))

(event EventBeginPlay
  (CallFunction|DisableTonemapper)
  (CallFunction|DisableEyeAdaptation))

(event Game|Damage|EventAnyDamage
  (params (Damage :type Float%20%28single-precision%29) (DamageType :type Damage%20Type%20Object%20Reference) (InstigatedBy :type Controller%20Object%20Reference) (DamageCauser :type Actor%20Object%20Reference))
  (bind _mesh (Variables|Character|GetMesh))
  (bind _health (CallFunction|DecreaseHealth Damage))
  (if (<= _health 0.0)
    (Variables|Default|SetDead? (<= _health 0.0))
    (Collision|SetActorEnableCollision false)
    (Pawn|Components|CharacterMovement|DisableMovement (Variables|Character|GetCharacterMovement))
    (Components|Animation|PlayAnimation _mesh "/Game/Characters/MainCharacter/Animations/Animations_Diying_Start.Animations_Diying_Start" false)
    (Utilities|FlowControl|Delay 1.0)
    (Components|Animation|PlayAnimation _mesh "/Game/Characters/MainCharacter/Animations/Animations_Diying_Loop.Animations_Diying_Loop" true)))

(fn ConstructionScript)

(fn DisableEyeAdaptation
  (Development|ExecuteConsoleCommand "ShowFlag.EyeAdaptation 0" 0)
  (Development|ExecuteConsoleCommand "r.EyeAdaptation.ExponentialTransitionDistance 0" 0)
  (Development|ExecuteConsoleCommand "r.EyeAdaptationQuality 0" 0))

(fn DisableTonemapper
  (Development|ExecuteConsoleCommand "ShowFlag.Tonemapper 0" 0)
  (Development|ExecuteConsoleCommand "r.TonemapperGamma 0" 0)
  (Development|ExecuteConsoleCommand "r.TonemapperFilm 0" 0)
  (Development|ExecuteConsoleCommand "r.Tonemapper.Sharpen 0" 0)
  (Development|ExecuteConsoleCommand "r.Tonemapper.GrainQuantization 0" 0)
  (Development|ExecuteConsoleCommand "r.Tonemapper.Quality 0" 0))

(fn DecreaseHealth
  (params (Damage%20Amount :type Float%20%28double-precision%29))
  (bind _output_get (Variables|Default|SetPlayer%20Health (- (Variables|Default|GetPlayer%20Health) Damage%20Amount)))
  (return _output_get))

(fn IsAlive
  (return (not (Variables|Default|GetDead?))))

(fn SpawnFireboll
  (if (CallFunction|IsAlive)
    (Animation|PlayAnimMontage "/Game/Characters/MainCharacter/Animations/Upper_Attack_Montage.Upper_Attack_Montage" 1.0 "None")
    (Game|SpawnActorfromClass "/Game/Visual_Effects/Fireboll_Actor.Fireboll_Actor_C" (Transformation|GetWorldTransform (Variables|Default|GetProjectileSpawn)) "Undefined" self 0)))

(fn SetPlayerCharacterDeath
  (params (Health%20Value :type Float%20%28double-precision%29))
  (Pawn|Components|CharacterMovement|DisableMovement (Variables|Character|GetCharacterMovement))
  (return))