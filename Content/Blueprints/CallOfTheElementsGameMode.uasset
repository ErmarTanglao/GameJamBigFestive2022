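; Game mode for CallOfTheElements that runs triggered enemy summon waves and tracks the spawned enemies.
; TriggerSummon spawns an enemy at once and starts a looping timer that spawns more at random Enemy_Spawn actors.
; When the spawn count runs out, it refills the count, stops the timer and resets the TriggerSummonAdds actor found at BeginPlay.
; RegisterEnemyDeath removes enemies from the list and checks wave completion, but that branch does nothing.
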(event Custom|Trigger%20Summon
  (Development|PrintString "Trigger activate")
  (Utilities|Time|SetTimerbyFunctionName 0 "Spawn Enemy" 2.0 true)
  (CallFunction|SpawnEnemy))

(event EventBeginPlay
  (bind _returnvalue (Actor|GetActorOfClass "/Game/Blueprints/TriggerSummonAdds.TriggerSummonAdds_C"))
  (Variables|Default|SetTrigger%20Summon%20Event%20Actor _returnvalue))

(fn ConstructionScript)

(fn SpawnEnemy
  (bind _spawn_point (CallFunction|GetRandomSpawnPoint))
  (Utilities|IsValid _spawn_point
    (:Is%20Valid
      (bind _returnvalue (Game|SpawnActorfromClass "/Game/Blueprints/EnemyCharacterBP.EnemyCharacterBP_C" (Transformation|GetActorTransform _spawn_point) "Undefined" 0 0))
      (Utilities|IsValid _returnvalue
        (:Is%20Valid
          (Utilities|Array|Add (Variables|Default|GetEnemys) _returnvalue)
          (bind _result (Math|Integer|DecrementInt (Variables|Default|GetEnemy%20Spawns%20Remaining))
            (:%20%20
              (Development|PrintString (Utilities|String|ToString(Integer) (Variables|Default|GetEnemy%20Spawns%20Remaining)))
              (if (== _result 0)
                (Variables|Default|SetEnemy%20Spawns%20Remaining 10)
                (Utilities|Time|ClearTimerbyFunctionName 0 "Spawn Enemy")
                (Default|ResetTriggerSummonAdds (Variables|Default|GetTrigger%20Summon%20Event%20Actor))))))))))

(fn GetRandomSpawnPoint
  (bind _outactors (Actor|GetAllActorsOfClass "/Game/Blueprints/Enemy_Spawn.Enemy_Spawn_C"))
  (return (Utilities|Array|Get(acopy) _outactors (Math|Random|RandomIntegerinRange 0 (Utilities|Array|LastIndex _outactors)))))

(fn RegisterEnemyDeath
  (params (Enemy :type Enemy%20Character%20BP%20Object%20Reference%20%28by%20ref%29))
  (Utilities|Array|RemoveItem (Variables|Default|GetEnemys) Enemy)
  (if (CallFunction|IsWaveComplete)
    _))

(fn IsWaveComplete
  (return (and (== (Utilities|Array|Length (Variables|Default|GetEnemys)) 0) (== (Variables|Default|GetEnemy%20Spawns%20Remaining) 0))))