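; Spell attack actor, likely a projectile, that triggers an impact when its collision sphere hits something.
; On BeginPlay it assigns the HitEffect asset to its Niagara component, Hiteffects.
; On hit it activates that component at the impact point, spawns an ImpactActor there and immediately destroys itself, along with the effect component it owns.
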(event OnComponentHit(CollisionSphere)
  (params (HitComponent :type Primitive%20Component%20Object%20Reference) (OtherActor :type Actor%20Object%20Reference) (OtherComp :type Primitive%20Component%20Object%20Reference) (NormalImpulse :type Vector :default "0, 0, 0") (Hit :type Hit%20Result%20Structure%20%28by%20ref%29))
  (bind _location (Collision|BreakHitResult Hit))
  (bind _hiteffects (Variables|Default|GetHiteffects))
  (Components|Activation|SetActive _hiteffects true false)
  (Transformation|SetWorldLocation _hiteffects _location false false)
  (Game|SpawnActorfromClass (Variables|Default|GetImpactActor) (Math|Transform|MakeTransform _location) "Undefined" 0 0)
  (Actor|DestroyActor))

(event EventBeginPlay
  (Class|NiagaraComponent|SetAsset (Variables|Default|GetHiteffects) (Variables|Default|GetHit%20Effect) true))

(fn ConstructionScript)