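; Player controller for MainCharacterBP, providing MMO-style third-person movement and camera controls through Enhanced Input.
; On BeginPlay it caches the pawn, adds the mapping context and sets Game-and-UI input with the cursor hidden.
; WASD or holding both mouse buttons moves the character, with forward following camera yaw.
; Q/E and right-mouse drag turn the camera with clamped pitch, and the scroll wheel zooms by clamping spring arm length.
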(event Input|EnhancedActionEvents|EnhancedInputActionMovementSides
  (params (ActionValue :type Float%20%28double-precision%29) (ElapsedSeconds :type Float%20%28double-precision%29) (TriggeredSeconds :type Float%20%28double-precision%29) (InputAction :type Input%20Action%20Object%20Reference :default "/Game/Blueprints/Input/Mouse/MovementSides.MovementSides"))
  ;[1 1 1] Character Movement WASD
  (:Triggered
    (CallFunction|MoveCharacterSide ActionValue)))

(event Input|EnhancedActionEvents|EnhancedInputActionMovementFrontBack
  (params (ActionValue :type Float%20%28double-precision%29) (ElapsedSeconds :type Float%20%28double-precision%29) (TriggeredSeconds :type Float%20%28double-precision%29) (InputAction :type Input%20Action%20Object%20Reference :default "/Game/Blueprints/Input/Mouse/MovementFrontBack.MovementFrontBack"))
  ;[1 1 1] Character Movement WASD
  (:Triggered
    (CallFunction|MoveCharacterFoward ActionValue)))

(event Input|EnhancedActionEvents|EnhancedInputActionQ-E_Rotation
  (params (ActionValue :type Float%20%28double-precision%29) (ElapsedSeconds :type Float%20%28double-precision%29) (TriggeredSeconds :type Float%20%28double-precision%29) (InputAction :type Input%20Action%20Object%20Reference :default "/Game/Blueprints/Input/Mouse/Q-E_Rotation.Q-E_Rotation"))
  ;[1 1 1] Rotate the Camera (Limited on Y axis)
  (:Triggered
    (CallFunction|RotationCameraXbyKeyboard ActionValue)))

(event Input|EnhancedActionEvents|EnhancedInputActionRightButtonHold
  (params (ActionValue :type Vector%202D%20Structure) (ElapsedSeconds :type Float%20%28double-precision%29) (TriggeredSeconds :type Float%20%28double-precision%29) (InputAction :type Input%20Action%20Object%20Reference :default "/Game/Blueprints/Input/Mouse/RightButtonHold.RightButtonHold"))
  ;[1 1 1] Rotate the Camera (Limited on Y axis)
  (:Triggered
    (CallFunction|RotationCamerainXAxisbyMouse (.x ActionValue))
    (CallFunction|RotationCamerainYAxisbyMouse (.y ActionValue))))

(event Input|EnhancedActionEvents|EnhancedInputActionLeftButtonPressed
  (params (ActionValue :type Float%20%28double-precision%29) (ElapsedSeconds :type Float%20%28double-precision%29) (TriggeredSeconds :type Float%20%28double-precision%29) (InputAction :type Input%20Action%20Object%20Reference :default "/Game/Blueprints/Input/Mouse/LeftButtonPressed.LeftButtonPressed"))
  ;[1 1 1] Move Pressing 2 mouse buttons
  (:Triggered
    (if (and (Variables|Default|GetLeft%20Mouse%20Button%20Held) (Variables|Default|GetRight%20Mouse%20Button%20Held))
      (CallFunction|MoveCharacterFoward ActionValue)))
  (:Started
    (Variables|Default|SetLeft%20Mouse%20Button%20Held true))
  (:Completed
    (Variables|Default|SetLeft%20Mouse%20Button%20Held false)))

(event Input|EnhancedActionEvents|EnhancedInputActionRightButtonPressed
  (params (ActionValue :type Vector%202D%20Structure) (ElapsedSeconds :type Float%20%28double-precision%29) (TriggeredSeconds :type Float%20%28double-precision%29) (InputAction :type Input%20Action%20Object%20Reference :default "/Game/Blueprints/Input/Mouse/RightButtonPressed.RightButtonPressed"))
  ;[1 1 1] Move Pressing 2 mouse buttons
  (:Started
    (Variables|Default|SetRight%20Mouse%20Button%20Held true))
  (:Completed
    (Variables|Default|SetRight%20Mouse%20Button%20Held false)))

(event Input|EnhancedActionEvents|EnhancedInputActionScroll
  (params (ActionValue :type Float%20%28double-precision%29) (ElapsedSeconds :type Float%20%28double-precision%29) (TriggeredSeconds :type Float%20%28double-precision%29) (InputAction :type Input%20Action%20Object%20Reference :default "/Game/Blueprints/Input/Mouse/Scroll.Scroll"))
  ;[1 1 1] Zoom using mouse scroll
  (:Triggered
    (CallFunction|ZoominandOutbyMouseScroll ActionValue)))

(event EventBeginPlay
  ;[1 1 1] Initial Settings
  (CallFunction|ReferencetoMainCharacter)
  (Input|SetInputModeGameandUI self 0 "DoNotLock" false false)
  (Class|PlayerController|AddPitchInput 2e+01)
  (Variables|Default|SetbShowMouseCursor false))

(fn ConstructionScript)

(fn ReferencetoMainCharacter
  (bind _asmain_character_bp (Utilities|Casting|CastToMainCharacterBP (Game|Player|GetPlayerPawn 0)))
  (Variables|Default|SetAs%20Main%20Character%20BP _asmain_character_bp)
  (Input|AddMappingContext (PlayerController|LocalPlayerSubsystems|GetEnhancedInputLocalPlayerSubsystem) 0 0 "(bIgnoreAllPressedKeysUntilRelease=True,bForceImmediately=False)"))

(fn RotationCamerainYAxisbyMouse
  (params (Y%20Mouse%20Value :type Float%20%28double-precision%29))
  (bind _returnvalue (Pawn|GetControlRotation :!class /Script/Engine.Controller))
  (Pawn|SetControlRotation (Math|Rotator|MakeRotator (.roll _returnvalue) (Math|Float|ClampAngle (+ (* (* (Utilities|Time|GetWorldDeltaSeconds) (Variables|Default|GetTurn%20Rate) Y%20Mouse%20Value) -1.0) (.pitch _returnvalue)) -5e+01 -1e+01) (.yaw _returnvalue))))

(fn RotationCamerainXAxisbyMouse
  (params (X%20Mouse%20Value :type Float%20%28double-precision%29))
  (Pawn|Input|AddControllerYawInput (Variables|Default|GetAs%20Main%20Character%20BP) (* X%20Mouse%20Value (Variables|Default|GetTurn%20Rate) (Utilities|Time|GetWorldDeltaSeconds))))

(fn RotationCameraXbyKeyboard
  (params (Val :type Float%20%28single-precision%29))
  (Pawn|Input|AddControllerYawInput (Variables|Default|GetAs%20Main%20Character%20BP) Val))

(fn ZoominandOutbyMouseScroll
  (params (Action%20Value :type Float%20%28double-precision%29))
  (bind _as_main_character_bp (Variables|Default|GetAs%20Main%20Character%20BP))
  (bind _springarm (Variables|/Game/Blueprints/MainCharacterBP.MainCharacterBP_C|GetSpringArm _as_main_character_bp))
  (Variables|/Script/Engine.SpringArmComponent|SetTargetArmLength _springarm (Math|Float|Clamp(Float) (+ (* Action%20Value 2e+01) (Variables|/Script/Engine.SpringArmComponent|GetTargetArmLength _springarm)) 1e+02 7e+02)))

(fn MoveCharacterFoward
  (params (ScaleValue :type Float%20%28single-precision%29))
  (Pawn|Input|AddMovementInput (Variables|Default|GetAs%20Main%20Character%20BP) (Math|Vector|GetForwardVector (Math|Rotator|MakeRotator 0.0 0.0 (.yaw (Pawn|GetControlRotation :!class /Script/Engine.Controller)))) ScaleValue false))

(fn MoveCharacterSide
  (params (ScaleValue :type Float%20%28single-precision%29))
  (bind _returnvalue (Transformation|GetActorRotation))
  (Pawn|Input|AddMovementInput (Variables|Default|GetAs%20Main%20Character%20BP) (Math|Vector|GetRightVector (Math|Rotator|MakeRotator (.roll _returnvalue) 0.0 (.yaw _returnvalue))) ScaleValue false))