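; EnemyCharacterBP is a character Blueprint that, despite its name, is driven by player input to move and cast four magic attacks.
; BeginPlay adds the GameJamInputMapping Enhanced Input context for player 0, and movement follows control rotation.
; Each attack input spawns its own BP_MagicAttack actor at the ProjectileSpawn transform.
; Logic to face the mouse cursor through a line trace exists but is disconnected and never runs.
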(event Input|EnhancedActionEvents|EnhancedInputActionIA_Attack1
  (params (ActionValue :type Boolean) (ElapsedSeconds :type Float%20%28double-precision%29) (TriggeredSeconds :type Float%20%28double-precision%29) (InputAction :type Input%20Action%20Object%20Reference :default "/Game/Blueprints/Input/IA_Attack1.IA_Attack1"))
  (:Triggered
    (Game|SpawnActorfromClass "/Game/Characters/MainCharacter/Blueprint/BP_MagicAttack1.BP_MagicAttack1_C" (Transformation|GetWorldTransform (Variables|Default|GetProjectileSpawn)) "AlwaysSpawn" 0 0)))

(event Input|EnhancedActionEvents|EnhancedInputActionIA_Movement
  (params (ActionValue :type Vector%202D%20Structure) (ElapsedSeconds :type Float%20%28double-precision%29) (TriggeredSeconds :type Float%20%28double-precision%29) (InputAction :type Input%20Action%20Object%20Reference :default "/Game/Blueprints/Input/IA_Movement.IA_Movement"))
  (bind _returnvalue (Pawn|GetControlRotation :!class /Script/Engine.Pawn))
  (bind _returnvalue_2 (Pawn|GetControlRotation :!class /Script/Engine.Pawn))
  (:Triggered
    (Pawn|Input|AddMovementInput (Math|Vector|GetRightVector (Math|Rotator|MakeRotator (.roll _returnvalue_2) 0.0 (.yaw _returnvalue_2))) (.x ActionValue) false)
    (Pawn|Input|AddMovementInput (Math|Vector|GetForwardVector (Math|Rotator|MakeRotator (.roll _returnvalue) 0.0 (.yaw _returnvalue))) (.y ActionValue) false)))

(event Input|EnhancedActionEvents|EnhancedInputActionIA_Attack2
  (params (ActionValue :type Boolean) (ElapsedSeconds :type Float%20%28double-precision%29) (TriggeredSeconds :type Float%20%28double-precision%29) (InputAction :type Input%20Action%20Object%20Reference :default "/Game/Blueprints/Input/IA_Attack2.IA_Attack2"))
  (:Triggered
    (Game|SpawnActorfromClass "/Game/Characters/MainCharacter/Blueprint/BP_MagicAttack2.BP_MagicAttack2_C" (Transformation|GetWorldTransform (Variables|Default|GetProjectileSpawn)) "AlwaysSpawn" 0 0)))

(event Input|EnhancedActionEvents|EnhancedInputActionIA_Attack3
  (params (ActionValue :type Boolean) (ElapsedSeconds :type Float%20%28double-precision%29) (TriggeredSeconds :type Float%20%28double-precision%29) (InputAction :type Input%20Action%20Object%20Reference :default "/Game/Blueprints/Input/IA_Attack3.IA_Attack3"))
  (:Triggered
    (Game|SpawnActorfromClass "/Game/Characters/MainCharacter/Blueprint/BP_MagicAttack3.BP_MagicAttack3_C" (Transformation|GetWorldTransform (Variables|Default|GetProjectileSpawn)) "AlwaysSpawn" 0 0)))

(event Input|EnhancedActionEvents|EnhancedInputActionIA_Attack4
  (params (ActionValue :type Boolean) (ElapsedSeconds :type Float%20%28double-precision%29) (TriggeredSeconds :type Float%20%28double-precision%29) (InputAction :type Input%20Action%20Object%20Reference :default "/Game/Blueprints/Input/IA_Attack4.IA_Attack4"))
  (:Triggered
    (Game|SpawnActorfromClass "/Game/Characters/MainCharacter/Blueprint/BP_MagicAttack4.BP_MagicAttack4_C" (Transformation|GetWorldTransform (Variables|Default|GetProjectileSpawn)) "AlwaysSpawn" 0 0)))

(event EventBeginPlay
  (bind _returnvalue (Game|GetPlayerController 0))
  (bind _returnvalue_2 (PlayerController|LocalPlayerSubsystems|GetEnhancedInputLocalPlayerSubsystem _returnvalue))
  (Utilities|IsValid _returnvalue_2
    (:Is%20Valid
      (Input|AddMappingContext _returnvalue_2 "/Game/Blueprints/Input/GameJamInputMapping.GameJamInputMapping" 0 "(bIgnoreAllPressedKeysUntilRelease=True,bForceImmediately=False)"))))

(event Collision|EventActorBeginOverlap
  (params (OtherActor :type Actor%20Object%20Reference)))

(event EventTick
  (params (DeltaSeconds :type Float%20%28single-precision%29)))

(fn ConstructionScript)