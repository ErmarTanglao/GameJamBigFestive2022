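; Player character Blueprint that fires four magic attacks from Enhanced Input actions.
; Each attack spawns its own projectile actor at the ProjectileSpawn transform with the character as Instigator.
; The first attack is always available, while the other three require the ObtainedBlue, ObtainedBrown and ObtainedGreen flags respectively.
; BeginPlay disables the tonemapper and eye adaptation through console commands.
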(event Input|EnhancedActionEvents|EnhancedInputActionIA_Attack1
  (params (ActionValue :type Boolean) (ElapsedSeconds :type Float%20%28double-precision%29) (TriggeredSeconds :type Float%20%28double-precision%29) (InputAction :type Input%20Action%20Object%20Reference :default "/Game/Blueprints/Input/IA_Attack1.IA_Attack1"))
  (:Triggered
    (Game|SpawnActorfromClass "/Game/Characters/MainCharacter/Blueprint/BP_MagicAttack1.BP_MagicAttack1_C" (Transformation|GetWorldTransform (Variables|Default|GetProjectileSpawn)) "AlwaysSpawn" 0 self)))

(event Input|EnhancedActionEvents|EnhancedInputActionIA_Attack2
  (params (ActionValue :type Boolean) (ElapsedSeconds :type Float%20%28double-precision%29) (TriggeredSeconds :type Float%20%28double-precision%29) (InputAction :type Input%20Action%20Object%20Reference :default "/Game/Blueprints/Input/IA_Attack2.IA_Attack2"))
  (:Triggered
    (if (Variables|Default|GetObtainedBlue)
      (Game|SpawnActorfromClass "/Game/Characters/MainCharacter/Blueprint/BP_MagicAttack2.BP_MagicAttack2_C" (Transformation|GetWorldTransform (Variables|Default|GetProjectileSpawn)) "AlwaysSpawn" 0 self))))

(event Input|EnhancedActionEvents|EnhancedInputActionIA_Attack3
  (params (ActionValue :type Boolean) (ElapsedSeconds :type Float%20%28double-precision%29) (TriggeredSeconds :type Float%20%28double-precision%29) (InputAction :type Input%20Action%20Object%20Reference :default "/Game/Blueprints/Input/IA_Attack3.IA_Attack3"))
  (:Triggered
    (if (Variables|Default|GetObtainedBrown)
      (Game|SpawnActorfromClass "/Game/Characters/MainCharacter/Blueprint/BP_MagicAttack3.BP_MagicAttack3_C" (Transformation|GetWorldTransform (Variables|Default|GetProjectileSpawn)) "AlwaysSpawn" 0 self))))

(event Input|EnhancedActionEvents|EnhancedInputActionIA_Attack4
  (params (ActionValue :type Boolean) (ElapsedSeconds :type Float%20%28double-precision%29) (TriggeredSeconds :type Float%20%28double-precision%29) (InputAction :type Input%20Action%20Object%20Reference :default "/Game/Blueprints/Input/IA_Attack4.IA_Attack4"))
  (:Triggered
    (if (Variables|Default|GetObtainedGreen)
      (Game|SpawnActorfromClass "/Game/Characters/MainCharacter/Blueprint/BP_MagicAttack4.BP_MagicAttack4_C" (Transformation|GetWorldTransform (Variables|Default|GetProjectileSpawn)) "AlwaysSpawn" 0 self))))

(event EventBeginPlay
  (CallFunction|DisableTonemapper)
  (CallFunction|DisableEyeAdaptation))

(fn ConstructionScript)

(fn DisableEyeAdaptation
  (Development|ExecuteConsoleCommand "ShowFlag.EyeAdaptation 0" 0)
  (Development|ExecuteConsoleCommand "r.EyeAdaptation.ExponentialTransitionDistance 0" 0)
  (Development|ExecuteConsoleCommand "r.EyeAdaptationQuality 0" 0))

(fn DisableTonemapper
  (Development|ExecuteConsoleCommand "ShowFlag.Tonemapper 0" 0)
  (Development|ExecuteConsoleCommand "r.TonemapperGamma 0" 0)
  (Development|ExecuteConsoleCommand "r.TonemapperFilm 0" 0)
  (Development|ExecuteConsoleCommand "r.Tonemapper.Sharpen 0" 0)
  (Development|ExecuteConsoleCommand "r.Tonemapper.GrainQuantization 0" 0)
  (Development|ExecuteConsoleCommand "r.Tonemapper.Quality 0" 0))