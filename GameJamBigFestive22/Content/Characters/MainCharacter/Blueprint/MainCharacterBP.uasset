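; Player character for a game jam game that moves on input, aims at the mouse cursor and fires magic attacks.
; BeginPlay adds the Enhanced Input mapping context, and the movement action drives movement along axes derived from control rotation.
; Each tick, a short cursor ray against WorldStatic objects sets the full actor rotation toward the impact point, without checking for a hit.
; The attack action spawns BP_MagicAttack at the ProjectileSpawn transform.
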(event Input|EnhancedActionEvents|EnhancedInputActionIA_Movement
  (params (ActionValue :type Vector%202D%20Structure) (ElapsedSeconds :type Float%20%28double-precision%29) (TriggeredSeconds :type Float%20%28double-precision%29) (InputAction :type Input%20Action%20Object%20Reference :default "/Game/Characters/MainCharacter/Input/IA_Movement.IA_Movement"))
  (bind _returnvalue (Pawn|GetControlRotation :!class /Script/Engine.Pawn))
  (bind _returnvalue_2 (Pawn|GetControlRotation :!class /Script/Engine.Pawn))
  (:Triggered
    (Pawn|Input|AddMovementInput (Math|Vector|GetRightVector (Math|Rotator|MakeRotator (.roll _returnvalue_2) 0.0 (.yaw _returnvalue_2))) (.x ActionValue) false)
    (Pawn|Input|AddMovementInput (Math|Vector|GetForwardVector (Math|Rotator|MakeRotator (.roll _returnvalue) 0.0 (.yaw _returnvalue))) (.y ActionValue) false)))

(event Input|EnhancedActionEvents|EnhancedInputActionIA_Attack
  (params (ActionValue :type Boolean) (ElapsedSeconds :type Float%20%28double-precision%29) (TriggeredSeconds :type Float%20%28double-precision%29) (InputAction :type Input%20Action%20Object%20Reference :default "/Game/Characters/MainCharacter/Input/IA_Attack.IA_Attack"))
  (:Triggered
    (Game|SpawnActorfromClass "/Game/Characters/MainCharacter/Blueprint/BP_MagicAttack.BP_MagicAttack_C" (Transformation|GetWorldTransform (Variables|Default|GetProjectileSpawn)) "AlwaysSpawn" 0 0)))

(event EventBeginPlay
  (bind _returnvalue (Game|GetPlayerController 0))
  (bind _returnvalue_2 (PlayerController|LocalPlayerSubsystems|GetEnhancedInputLocalPlayerSubsystem _returnvalue))
  (Utilities|IsValid _returnvalue_2
    (:Is%20Valid
      (Input|AddMappingContext _returnvalue_2 "/Game/Characters/MainCharacter/Input/GameJamInputMapping.GameJamInputMapping" 0 "(bIgnoreAllPressedKeysUntilRelease=True,bForceImmediately=False)"))))

(event Collision|EventActorBeginOverlap
  (params (OtherActor :type Actor%20Object%20Reference)))

(event EventTick
  (params (DeltaSeconds :type Float%20%28single-precision%29))
  (bind _returnvalue (Game|GetPlayerController 0))
  (bind (_worldlocation _worlddirection) (Game|Player|ConvertMouseLocationToWorldSpace _returnvalue))
  (bind _outhit (Collision|LineTraceForObjects _worldlocation (+ _worldlocation (* _worlddirection "1000.000000,1000.000000,1000.000000")) (Utilities|Array|MakeArray "ObjectTypeQuery1") false 0 "None"))
  (Transformation|SetActorRotation (Math|Rotator|FindLookatRotation (Transformation|GetActorLocation) (.ImpactPoint (Collision|BreakHitResult _outhit)))))

(fn ConstructionScript)